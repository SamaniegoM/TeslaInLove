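; BP_GI_Dialogue manages NPC conversations, showing one line of text at a time.
; TryStartDialoge rejects empty line arrays, otherwise stores the lines and NPC, creates or reuses a WB_Dialogue widget and disables Bp_Player movement.
; AdvanceDialogue steps through the lines, updating the widget and passing each index to the NPC's Reaction.
; After the last line, EndDialogue removes the widget, clears state and restores movement.
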(fn AdvanceDialogue
  (if (Variables|Default|GetbDialogueActive)
    (bind _output_get (Variables|Default|SetTalkIndex (+ (Variables|Default|GetTalkIndex) 1)))
    (if (< _output_get (Utilities|Array|Length (Variables|Default|GetCurrentLines)))
      (Default|SetLine (Variables|Default|GetUi) (Utilities|Array|Get(acopy) (Variables|Default|GetCurrentLines) (Variables|Default|GetTalkIndex)))
      (Default|Reaction (Variables|Default|GetcurrentNpc) (Variables|Default|GetTalkIndex))
      (else
        (CallFunction|EndDialogue)))
    (return)
    (else
      (return))))

(fn TryStartDialoge
  (params (Lines :type Array%20of%20Texts) (Pc :type Player%20Controller%20Object%20Reference) (currentNpc :type BP%20Npc%20Object%20Reference))
  (if (> (Utilities|Array|Length Lines) 0)
    (Variables|Default|SetcurrentNpc currentNpc)
    (Variables|Default|SetCurrentLines Lines)
    (Variables|Default|SetTalkIndex 0)
    (Variables|Default|SetbDialogueActive true)
    (if (Utilities|IsValid (Variables|Default|GetUi))
      _
      (else
        (bind _returnvalue (UserInterface|CreateWidget "/Game/Blueprint/Npc/WB_Dialogue.WB_Dialogue_C" Pc))
        (bind _output_get (Variables|Default|SetUi _returnvalue))))
    (UserInterface|Viewport|AddtoViewport _output_get 0)
    (bind _asbp_player (Utilities|Casting|CastToBp_Player (Game|GetPlayerCharacter 0)))
    (Variables|/Game/Blueprint/Bp_Player.Bp_Player_C|SetCanMove _asbp_player false)
    (Default|SetLine (Variables|Default|GetUi) (Utilities|Array|Get(acopy) (Variables|Default|GetCurrentLines) (Variables|Default|GetTalkIndex)))
    (Default|Reaction (Variables|Default|GetcurrentNpc) (Variables|Default|GetTalkIndex))
    (return true)
    (else
      (return false))))

(fn EndDialogue
  (Widget|RemovefromParent (Variables|Default|GetUi))
  (Variables|Default|SetbDialogueActive false)
  (Utilities|Array|Clear (Variables|Default|GetCurrentLines))
  (Variables|Default|SetTalkIndex 0)
  (bind _asbp_player (Utilities|Casting|CastToBp_Player (Game|GetPlayerCharacter 0)))
  (Variables|/Game/Blueprint/Bp_Player.Bp_Player_C|SetCanMove _asbp_player true))