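; Player Blueprint for point-and-click movement, interaction and pausing, with the mouse cursor shown.
; Left click, gated by CanMove, traces from the cursor with debug drawing and moves to the hit point via SimpleMoveToLocation.
; Releasing E messages overlapping actors through BPI_Interactive, or BPI_Dialog for those without it.
; F toggles pause, reusing a lazily created BP_Pause widget and switching input modes.
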(event EventBeginPlay
  (Variables|/Script/Engine.PlayerController|SetbShowMouseCursor (Game|GetPlayerController 0) true))

(event Input|KeyboardEvents|E
  (params (Key :type Key%20Structure :default "None"))
  (:Released
    (for _array_element (Collision|GetOverlappingActors 0 :!class /Script/Engine.Actor)
      (if (Utilities|DoesObjectImplementInterface _array_element "/Game/Blueprint/Minigame/BPI_Interactive.BPI_Interactive_C")
        (Class|BPIInteractive|Interact(Message) _array_element)
        (elif (Utilities|DoesObjectImplementInterface _array_element "/Game/Blueprint/Npc/BPI_Dialog.BPI_Dialog_C")
          (Class|BPIDialog|Talk(Message) _array_element))))))

(event Input|MouseEvents|LeftMouseButton
  (params (Key :type Key%20Structure :default "None"))
  (bind _returnvalue (Game|GetPlayerController 0))
  (bind (_worldlocation _worlddirection) (Game|Player|ConvertMouseLocationToWorldSpace _returnvalue))
  (:Pressed
    (if (Variables|Default|GetCanMove)
      (bind (_outhit _returnvalue_2) (Collision|LineTraceByChannel _worldlocation (+ _worldlocation (* _worlddirection 1e+04)) "TraceTypeQuery1" false 0 "ForDuration"))
      (if _returnvalue_2
        (AI|Navigation|SimpleMovetoLocation (Pawn|GetController) (.Location (Collision|BreakHitResult _outhit)))))))

(event Input|KeyboardEvents|F
  (params (Key :type Key%20Structure :default "None"))
  (bind _returnvalue (Game|GetPlayerController 0))
  ;[0.15 0.15 0.15 0.5] Pause Game
  (:Pressed
    (Utilities|IsValid (Variables|Default|GetPause%20Ref)
      (:Is%20Valid
        _)
      (:Is%20Not%20Valid
        (bind _returnvalue_2 (UserInterface|CreateWidget "/Game/Blueprint/Menus/BP_Pause.BP_Pause_C"))
        (Variables|Default|SetPause%20Ref _returnvalue_2)))
    (if (Game|IsGamePaused)
      (Widget|RemovefromParent (Variables|Default|GetPause%20Ref))
      (Game|SetGamePaused false)
      (Input|SetInputModeGameOnly _returnvalue false)
      (else
        (Game|SetGamePaused true)
        (UserInterface|Viewport|AddtoViewport (Variables|Default|GetPause%20Ref) 0)
        (Input|SetInputModeUIOnly _returnvalue (Variables|Default|GetPause%20Ref) "DoNotLock" false)))))

(fn ConstructionScript)