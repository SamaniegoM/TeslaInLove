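; Interactable minigame Blueprint that opens what appears to be a pipe puzzle and opens a linked door when it is solved.
; Interact creates WBP_MinigameUI, passing itself as parent along with the pipe row setting, then adds it to the viewport and disables player movement.
; CloseMinigame removes the widget and restores movement, while PuzzleCompleted only calls OpenDoor on DoorRef.
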(event Custom|Close%20Minigame
  (bind _wbp_ui (Variables|Default|GetWBP_UI))
  (Utilities|IsValid _wbp_ui
    (:Is%20Valid
      (Widget|RemovefromParent _wbp_ui)
      (bind _asbp_player (Utilities|Casting|CastToBp_Player (Game|GetPlayerCharacter 0)))
      (Variables|/Game/Blueprint/Bp_Player.Bp_Player_C|SetCanMove _asbp_player true))))

(event Custom|PuzzleCompleted
  (Default|OpenDoor (Variables|Default|GetDoorRef)))

(event EventInteract
  (bind _returnvalue (UserInterface|CreateWidget "/Game/Blueprint/Minigame/WBP_MinigameUI.WBP_MinigameUI_C" (Game|GetPlayerController 0) self (Variables|Default|GetpipeRows)))
  (bind _output_get (Variables|Default|SetWBP_UI _returnvalue))
  (UserInterface|Viewport|AddtoViewport _output_get 0)
  (bind _asbp_player (Utilities|Casting|CastToBp_Player (Game|GetPlayerCharacter 0)))
  (Variables|/Game/Blueprint/Bp_Player.Bp_Player_C|SetCanMove _asbp_player false))

(fn ConstructionScript)